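; BP_arkanoid is an Arkanoid-style block field that scores and removes pieces when they are hit.
; The construction script builds a grid of static mesh components from X, Y and spacing variables; the X loop subtracts -1, running to X+1 rather than X-1.
; On Hit, it adds a fixed score to the first BP_counter found in the level and destroys the struck component.
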(event Collision|EventHit
  (params (MyComp :type Primitive%20Component%20Object%20Reference) (Other :type Actor%20Object%20Reference) (OtherComp :type Primitive%20Component%20Object%20Reference) (bSelfMoved :type Boolean) (HitLocation :type Vector :default "0, 0, 0") (HitNormal :type Vector :default "0, 0, 0") (NormalImpulse :type Vector :default "0, 0, 0") (Hit :type Hit%20Result%20Structure%20%28by%20ref%29))
  (bind _outactors (Actor|GetAllActorsOfClass "/Game/MyProfectKymis/Arcanoid/BP_counter.BP_counter_C"))
  (Variables|/Game/MyProfectKymis/Arcanoid/BP_counter.BP_counter_C|SetCount (Utilities|Array|Get(acopy) _outactors) (+ (Variables|/Game/MyProfectKymis/Arcanoid/BP_counter.BP_counter_C|GetCount (Utilities|Array|Get(acopy) _outactors)) 10))
  (Components|DestroyComponent MyComp))

(fn ConstructionScript
  (for _index (range 0 (- (Variables|Default|GetX) -1))
    (for _index_2 (range 0 (- (Variables|Default|GetY) 1))
      (AddComponent|AddStaticMeshComponent false (Math|Transform|MakeTransform (Math|Vector|MakeVector (Math|Conversions|ToFloat(Integer) (* _index (Variables|Default|GetXDistance))) (Math|Conversions|ToFloat(Integer) (* _index_2 (Variables|Default|GetYDistance))) 0.0))))))