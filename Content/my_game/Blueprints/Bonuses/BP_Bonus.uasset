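; BP_Bonus is a moving bonus actor that gets one of two random types and displays that type as text.
; The Construction Script picks the BonucType enum value at random and writes its name to a TextRender.
; Each Tick applies a swept world offset from Speed, Direction and delta time, using only the X component, so it moves along world X.
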(event EventTick
  (params (DeltaSeconds :type Float%20%28single-precision%29))
  (Transformation|AddActorWorldOffset (Math|Vector|MakeVector (.x (* (* DeltaSeconds (Variables|Default|GetSpeed)) (Variables|Default|GetDirection))) 0.0 0.0) true))

(fn ConstructionScript
  (Variables|Default|SetBonucType (Utilities|Select :Index (Math|Random|RandomIntegerinRange 0 1) :Option%200 "NewEnumerator0" :Option%201 "NewEnumerator1"))
  (Rendering|Components|TextRender|SetText (Variables|Default|GetTextRender) (Utilities|Text|ToText(String) (Utilities|String|EnumtoString (Variables|Default|GetBonucType)))))