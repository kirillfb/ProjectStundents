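; BP_Cube_child is a cube actor that spawns a bonus when destroyed, if it starts with a gold material.
; On BeginPlay it checks the Cube's first material against MI_Metal_Gold and only then binds SpawnBonuc to its OnDestroyed event.
; That handler always spawns an actor at the cube's location with a fixed rotation, ignoring collisions.
; The construction script only calls the parent's.
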(event Custom|SpawnBonuc
  (params (DestroyedActor :type Actor%20Object%20Reference))
  (Game|SpawnActorfromClass "/Game/my_game/Blueprints/Bonuses/BP_Bonus.BP_Bonus_C" (Math|Transform|MakeTransform (Transformation|GetActorLocation) "-90.000000,0.000000,0.000000") "AlwaysSpawn" "MultiplyWithRoot" 0 0))

(event EventBeginPlay
  (if (== (Rendering|Material|GetMaterial (Variables|Default|GetCube) 0) "/Game/my_game/Material/Metalls/MI_Metal_Gold.MI_Metal_Gold")
    (Game|BindEventtoOnDestroyed (delegate Custom|SpawnBonuc))))

(fn ConstructionScript
  (|CallParentFunction))