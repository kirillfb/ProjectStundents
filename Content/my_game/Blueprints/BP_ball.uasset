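; BP_ball is a ball actor that moves in the X-Y plane and bounces off whatever blocks it.
; Each Tick it makes a swept world offset from Speed, Direction and delta time.
; On a blocking hit it reflects Direction about the surface normal.
; It also adds AdedSpeed to Speed, capped at 4000, but only when Speed is below zero.
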(event EventTick
  (params (DeltaSeconds :type Float%20%28single-precision%29))
  (bind _sweephitresult (Transformation|AddActorWorldOffset (Math|Vector|MakeVector (.x (* (* (Variables|Default|Getspeed) DeltaSeconds) (Variables|Default|GetDirection))) (.y (* (* (Variables|Default|Getspeed) DeltaSeconds) (Variables|Default|GetDirection))) 0.0) true))
  (if (.bBlockingHit (Collision|BreakHitResult _sweephitresult))
    (Variables|Default|SetDirection (Math|Vector|GetReflectionVector (Variables|Default|GetDirection) (.Normal (Collision|BreakHitResult _sweephitresult))))
    (if (< (Variables|Default|Getspeed) 0.0)
      (Variables|Default|Setspeed (Math|Float|Min(Float) (+ (Variables|Default|Getspeed) (Variables|Default|Getaded%20speed)) 4e+03)))))

(fn ConstructionScript)