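; BP_Cubes_generator is an actor that spawns a padded X-by-Y grid of BP_Cube_child actors from its location.
; The construction script builds a static-mesh preview, looping one Y step further than the spawn, which BeginPlay destroys before spawning.
; Spawned cubes fill CubesArray, whose length becomes AmountCubes through GetCubesForWin.
; An OnDestroyed binding runs per cube without using the element, and its CubeDead handler is empty.
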(event Custom|CubeDead
  (params (DestroyedActor :type Actor%20Object%20Reference)))

(event EventBeginPlay
  (bind _returnvalue (Transformation|GetActorLocation))
  (for _array_element (Variables|Default|GetPreview%20array)
    (Components|DestroyComponent _array_element))
  (for _index (range 1 (- (Variables|Default|GetX) 1))
    (for _index_2 (range 0 (- (Variables|Default|GetY) 1))
      (bind _returnvalue_2 (Game|SpawnActorfromClass "/Game/my_game/Blueprints/BP_Cube_child.BP_Cube_child_C" (Math|Transform|MakeTransform (Math|Vector|MakeVector (+ (.x _returnvalue) (Math|Conversions|ToFloat(Integer) (* _index (Variables|Default|GetPadding)))) (+ (.y _returnvalue) (Math|Conversions|ToFloat(Integer) (* _index_2 (Variables|Default|GetPadding)))) (.z _returnvalue))) "Undefined" "MultiplyWithRoot" 0 0))
      (Utilities|Array|Add (Variables|Default|GetCubesArray) _returnvalue_2)))
  (bind _amount_cubes (CallFunction|GetCubesforWin))
  (Variables|Default|SetAmount%20Cubes _amount_cubes)
  (for _array_element_2 (Variables|Default|GetCubesArray)
    (Game|BindEventtoOnDestroyed (delegate Custom|CubeDead))))

(fn ConstructionScript
  (for _index (range 1 (- (Variables|Default|GetX) 1))
    (for _index_2 (range 0 (Variables|Default|GetY))
      (bind _returnvalue (AddComponent|AddStaticMeshComponent false (Math|Transform|MakeTransform (Math|Vector|MakeVector (Math|Conversions|ToFloat(Integer) (* _index (Variables|Default|GetPadding))) (Math|Conversions|ToFloat(Integer) (* _index_2 (Variables|Default|GetPadding))) 0.0))))
      (Utilities|Array|Add (Variables|Default|GetPreview%20array) _returnvalue))))

(fn GetCubesforWin
  (return (Utilities|Array|Length (Variables|Default|GetCubesArray))))