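; Player controller that drives a BP_MyPown pawn and sets up the player's HUD.
; BeginPlay switches to game-only input, then creates WBP_Hud, adds it to the viewport and stores it.
; On possession it caches the pawn, which the Left_Right axis slides along world Y with a swept, delta-time-scaled offset.
; The SpawnBall action calls SpawnBall on that pawn.
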(event EventPossess
  (params (PossessedPawn :type Pawn%20Object%20Reference))
  (bind _asbp_my_pown (Utilities|Casting|CastToBP_MyPown PossessedPawn))
  (Variables|Default|SetMyPown _asbp_my_pown))

(event EventBeginPlay
  (Input|SetInputModeGameOnly self false)
  (bind _returnvalue (UserInterface|CreateWidget "/Game/my_game/WBP_Hud.WBP_Hud_C" self))
  (UserInterface|Viewport|AddtoViewport _returnvalue 0)
  (Variables|Default|SetHUD _returnvalue))

(event Input|ActionEvents|InputActionSpawnBall
  (params (Key :type Key%20Structure :default "None"))
  (:Pressed
    (Default|SpawnBall (Variables|Default|GetMyPown))))

(event Input|AxisEvents|InputAxisLeft_Right
  (params (AxisValue :type Float%20%28single-precision%29))
  (Transformation|AddActorWorldOffset (Variables|Default|GetMyPown) (Math|Vector|MakeVector 0.0 (* AxisValue (Utilities|Time|GetWorldDeltaSeconds) (Variables|Default|GetSpeed)) 0.0) true))

(fn ConstructionScript)