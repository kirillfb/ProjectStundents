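; Player pawn for a ball game, with a Cube body that catches bonuses, a life counter and ball spawning.
; SpawnBall launches one tracked BP_ball at the Arrow while lives remain; its destruction costs a life, broadcasting LivesChange and, at zero, GameOver.
; Overlapping a BP_Bonus destroys it and either spawns a smaller extra actor or widens the Cube, with a retriggerable delay restoring its saved scale.
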(event OnComponentBeginOverlap(Cube)
  (params (OverlappedComponent :type Primitive%20Component%20Object%20Reference) (OtherActor :type Actor%20Object%20Reference) (OtherComp :type Primitive%20Component%20Object%20Reference) (OtherBodyIndex :type Integer) (bFromSweep :type Boolean) (SweepResult :type Hit%20Result%20Structure%20%28by%20ref%29))
  (bind _asbp_bonus (Utilities|Casting|CastToBP_Bonus OtherActor))
  (switch Utilities|FlowControl|Switch|SwitchonE_BonusType (Variables|/Game/my_game/Blueprints/Bonuses/BP_Bonus.BP_Bonus_C|GetBonucType _asbp_bonus)
    (:NewEnumerator0
      (CallFunction|Max))
    (:NewEnumerator1
      (CallFunction|Ball)))
  (Actor|DestroyActor _asbp_bonus))

(event Custom|SpawnBall
  (if (not (<= (Variables|Default|GetPlayerLives) 0))
    (Variables|Default|GetAliveBall
      (:then)
      (:else
        (bind _returnvalue (Game|SpawnActorfromClass "/Game/my_game/Blueprints/BP_ball.BP_ball_C" (Math|Transform|MakeTransform (Transformation|GetWorldLocation (Variables|Default|GetArrow))) "Undefined" "MultiplyWithRoot" 0 0))
        (bind _output_get (Variables|Default|SetAliveBall _returnvalue))
        (Game|BindEventtoOnDestroyed _output_get (delegate Custom|BallsDead))))))

(event Custom|BallsDead
  (params (DestroyedActor :type Actor%20Object%20Reference))
  (bind _result (Math|Integer|DecrementInt (Variables|Default|GetPlayerLives))
    (:%20%20
      (Default|CallLivesChange _result)
      (if (<= _result 0)
        (Default|CallGameOver)))))

(event Custom|Max
  (bind _cube (Variables|Default|GetCube))
  (bind _relativescale3d (Variables|/Script/Engine.SceneComponent|GetRelativeScale3D _cube))
  (Transformation|SetRelativeScale3D _cube (Math|Vector|MakeVector (.x _relativescale3d) (* (.y _relativescale3d) 1.2) (.z _relativescale3d)))
  (CallFunction|MIN))

(event Custom|LiveEvent
  (bind _result (Math|Integer|IncrementInt (Variables|Default|GetPlayerLives))
    (:%20%20
      (Default|CallLivesChange _result))))

(event Custom|Ball
  (Game|SpawnActorfromClass "/Game/my_game/Blueprints/BP_ball.BP_ball_C" (Math|Transform|MakeTransform (Transformation|GetWorldLocation (Variables|Default|GetArrow)) "0, 0, 0" "0.700000,0.700000,0.700000") "Undefined" "MultiplyWithRoot" 0 0))

(event Custom|MIN
  (Utilities|FlowControl|RetriggerableDelay 2.0)
  (Transformation|SetRelativeScale3D (Variables|Default|GetCube) (Variables|Default|GetDefay%20scale)))

(event EventBeginPlay
  (Variables|Default|SetDefay%20scale (Variables|/Script/Engine.SceneComponent|GetRelativeScale3D (Variables|Default|GetCube))))

(fn ConstructionScript)