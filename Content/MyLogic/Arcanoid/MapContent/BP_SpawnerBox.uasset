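; BP_SpawnerBox builds the brick field for an Arkanoid game and handles bricks being hit.
; The construction script lays out a configurable X by Y grid of static mesh components with adjustable spacing, all within one actor.
; Its Hit event destroys the passed component and adds points to the BP_Global game instance.
; Chained random rolls then occasionally spawn a BP_Bonus or, failing that, a BP_Debuf at the hit location.
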(event Collision|EventHit
  (params (MyComp :type Primitive%20Component%20Object%20Reference) (Other :type Actor%20Object%20Reference) (OtherComp :type Primitive%20Component%20Object%20Reference) (bSelfMoved :type Boolean) (HitLocation :type Vector :default "0, 0, 0") (HitNormal :type Vector :default "0, 0, 0") (NormalImpulse :type Vector :default "0, 0, 0") (Hit :type Hit%20Result%20Structure%20%28by%20ref%29))
  (bind _returnvalue (Math|Random|RandomIntegerinRange 0 9))
  (Components|DestroyComponent MyComp)
  (bind _asbp_global (Utilities|Casting|CastToBP_Global (Game|GetGameInstance)))
  (Variables|/Game/MyLogic/Arcanoid/BP_Global.BP_Global_C|SetPoints _asbp_global (+ (Variables|/Game/MyLogic/Arcanoid/BP_Global.BP_Global_C|GetPoints _asbp_global) 10))
  (if (== _returnvalue 9)
    (Game|SpawnActorfromClass "/Game/MyLogic/Arcanoid/MapContent/BP_Bonus.BP_Bonus_C" (Math|Conversions|ToTransform(Vector) HitLocation) "Undefined" 0 0)
    (elif (== _returnvalue 8)
      (Game|SpawnActorfromClass "/Game/MyLogic/Arcanoid/MapContent/BP_Debuf.BP_Debuf_C" (Math|Conversions|ToTransform(Vector) HitLocation) "Undefined" 0 0))))

(fn ConstructionScript
  (for _index (range 0 (- (Variables|Default|GetX) 1))
    (for _index_2 (range 0 (- (Variables|Default|GetY) 1))
      (AddComponent|AddStaticMeshComponent false (Math|Transform|MakeTransform (Math|Vector|MakeVector (Math|Conversions|ToFloat(Integer) (* _index (Variables|Default|GetXdistance))) (Math|Conversions|ToFloat(Integer) (* _index_2 (Variables|Default|GetYdistance))) 0.0))))))