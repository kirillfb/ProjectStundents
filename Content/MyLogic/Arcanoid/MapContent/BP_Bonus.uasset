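; BP_Bonus is a moving Arcanoid bonus that turns into two extra balls when hit.
; Tick moves it along its direction with a swept offset and reflects that direction off the surface normal on blocking hits.
; Its Hit event destroys the bonus, spawns two BP_Ball actors randomly jittered around the hit location, and adds two to BallCount in the BP_Global game instance.
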(event Collision|EventHit
  (params (MyComp :type Primitive%20Component%20Object%20Reference) (Other :type Actor%20Object%20Reference) (OtherComp :type Primitive%20Component%20Object%20Reference) (bSelfMoved :type Boolean) (HitLocation :type Vector :default "0, 0, 0") (HitNormal :type Vector :default "0, 0, 0") (NormalImpulse :type Vector :default "0, 0, 0") (Hit :type Hit%20Result%20Structure%20%28by%20ref%29))
  (Actor|DestroyActor)
  (for _index (range 0 1)
    (Game|SpawnActorfromClass "/Game/MyLogic/Arcanoid/MapContent/BP_Ball.BP_Ball_C" (Math|Transform|MakeTransform (Math|Vector|MakeVector (+ (.x HitLocation) (Math|Random|RandomFloatinRange -2.0 2.0)) (+ (.y HitLocation) (Math|Random|RandomFloatinRange -2.0 2.0)) (.z HitLocation)) "0, 0, 0" "1,1,1") "Undefined" 0 0))
  (bind _asbp_global (Utilities|Casting|CastToBP_Global (Game|GetGameInstance)))
  (Variables|/Game/MyLogic/Arcanoid/BP_Global.BP_Global_C|SetBallCount _asbp_global (+ (Variables|/Game/MyLogic/Arcanoid/BP_Global.BP_Global_C|GetBallCount _asbp_global) 2)))

(event EventTick
  (params (DeltaSeconds :type Float%20%28single-precision%29))
  (bind _sweephitresult (Transformation|AddActorWorldOffset (* (* (Variables|Default|Getdirection) (Variables|Default|Getspeed)) DeltaSeconds) true))
  (if (.bBlockingHit (Collision|BreakHitResult _sweephitresult))
    (Variables|Default|Setdirection (Math|Vector|GetReflectionVector (Math|Vector|MakeVector (.x (Variables|Default|Getdirection)) (.y (Variables|Default|Getdirection)) 0.0) (.Normal (Collision|BreakHitResult _sweephitresult))))))

(fn ConstructionScript)