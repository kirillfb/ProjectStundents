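; BP_Debuf is a moving debuff pickup that shrinks the platform it hits.
; Tick moves it along Direction at Speed with a swept offset and reflects Direction off the surface normal on a blocking hit.
; The Hit event destroys the actor regardless of what it struck, then, for a BP_Platrorm, reduces the platform mesh's X scale by a fixed step unless it is already below a minimum threshold.
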(event Collision|EventHit
  (params (MyComp :type Primitive%20Component%20Object%20Reference) (Other :type Actor%20Object%20Reference) (OtherComp :type Primitive%20Component%20Object%20Reference) (bSelfMoved :type Boolean) (HitLocation :type Vector :default "0, 0, 0") (HitNormal :type Vector :default "0, 0, 0") (NormalImpulse :type Vector :default "0, 0, 0") (Hit :type Hit%20Result%20Structure%20%28by%20ref%29))
  (Actor|DestroyActor)
  (bind _asbp_platrorm (Utilities|Casting|CastToBP_Platrorm Other))
  (if (not (< (.x (Variables|/Script/Engine.SceneComponent|GetRelativeScale3D (Variables|/Game/MyLogic/Task_1/BP_Platrorm.BP_Platrorm_C|GetPlatform _asbp_platrorm))) 4.0))
    (Transformation|SetRelativeScale3D (Variables|/Game/MyLogic/Task_1/BP_Platrorm.BP_Platrorm_C|GetPlatform _asbp_platrorm) (Math|Vector|MakeVector (- (.x (Variables|/Script/Engine.SceneComponent|GetRelativeScale3D (Variables|/Game/MyLogic/Task_1/BP_Platrorm.BP_Platrorm_C|GetPlatform _asbp_platrorm))) 3.0) (.y (Variables|/Script/Engine.SceneComponent|GetRelativeScale3D (Variables|/Game/MyLogic/Task_1/BP_Platrorm.BP_Platrorm_C|GetPlatform _asbp_platrorm))) (.z (Variables|/Script/Engine.SceneComponent|GetRelativeScale3D (Variables|/Game/MyLogic/Task_1/BP_Platrorm.BP_Platrorm_C|GetPlatform _asbp_platrorm)))))))

(event EventTick
  (params (DeltaSeconds :type Float%20%28single-precision%29))
  (bind _sweephitresult (Transformation|AddActorWorldOffset (* (* (Variables|Default|Getdirection) (Variables|Default|Getspeed)) DeltaSeconds) true))
  (if (.bBlockingHit (Collision|BreakHitResult _sweephitresult))
    (Variables|Default|Setdirection (Math|Vector|GetReflectionVector (Math|Vector|MakeVector (.x (Variables|Default|Getdirection)) (.y (Variables|Default|Getdirection)) 0.0) (.Normal (Collision|BreakHitResult _sweephitresult))))))

(fn ConstructionScript)