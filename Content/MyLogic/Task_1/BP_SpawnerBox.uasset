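; BP_SpawnerBox is a grid of mesh boxes that break when hit and spawn bonus pickups.
; The construction script builds an X by Y grid of static mesh components spaced by Xdistance and Ydistance.
; On Hit, it destroys the struck component and spawns two BP_Bonus actors at the root's transform, not the broken box's.
; The random check before each spawn has a zero-only range, so it always passes.
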(event Collision|EventHit
  (params (MyComp :type Primitive%20Component%20Object%20Reference) (Other :type Actor%20Object%20Reference) (OtherComp :type Primitive%20Component%20Object%20Reference) (bSelfMoved :type Boolean) (HitLocation :type Vector :default "0, 0, 0") (HitNormal :type Vector :default "0, 0, 0") (NormalImpulse :type Vector :default "0, 0, 0") (Hit :type Hit%20Result%20Structure%20%28by%20ref%29))
  (Components|DestroyComponent MyComp)
  (for _index (range 0 1)
    (if (== (Math|Random|RandomIntegerinRange 0 0) 0)
      (Game|SpawnActorfromClass "/Game/MyLogic/Task_1/BP_Bonus.BP_Bonus_C" (Transformation|GetWorldTransform (Variables|Default|GetDefaultSceneRoot)) "Undefined" 0 0))))

(fn ConstructionScript
  (for _index (range 0 (- (Variables|Default|GetX) 1))
    (for _index_2 (range 0 (- (Variables|Default|GetY) 1))
      (AddComponent|AddStaticMeshComponent false (Math|Transform|MakeTransform (Math|Vector|MakeVector (Math|Conversions|ToFloat(Integer) (* _index (Variables|Default|GetXdistance))) (Math|Conversions|ToFloat(Integer) (* _index_2 (Variables|Default|GetYdistance))) 0.0))))))